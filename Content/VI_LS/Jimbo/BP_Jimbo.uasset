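; BP_Jimbo is a talking character actor with a screen face, driven by control messages through VI_GameInstance.
; On websocket connect it sends its generated actions JSON.
; "Speak" control messages trigger a TTS request to a local server, and the returned SoundWave plays on its Audio component.
; Each tick it feeds FaceWidget's render target into the face screen's dynamic material.
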(event Custom|OnCtrl
  (params (ControlMessage :type Control%20Message%20Base%20Structure%20%28by%20ref%29))
  (if (Utilities|Enum|Equal(Enum) (.type ControlMessage) "control")
    (if (Utilities|Enum|Equal(Enum) (.action (.speakpayload ControlMessage)) "speak")
      (Class|VIGameInstance|RequestforTTS (Variables|Default|GetVI_GameInstance) (.content (.speakpayload ControlMessage)) "http://127.0.0.1:8192/tts_speak" "2"))))

(event Custom|TTSFeedback
  (params (TTSFeedback :type TTS%20Feedback%20Structure%20%28by%20ref%29))
  (bind _audio (Variables|Default|GetAudio))
  (Audio|Components|Audio|SetSound _audio (.soundwave TTSFeedback))
  (Audio|Components|Audio|Play _audio 0.0))

(event Custom|OnConnect
  (params (bConnectSuccess :type Boolean))
  (if bConnectSuccess
    (bind _returnvalue (Class|VICharacterBase|GenerateActionsJSON "set"))
    (Class|VIGameInstance|SendMessageViaSocket (Variables|Default|GetVI_GameInstance) _returnvalue)))

(event Custom|TestAnimationWorks
  (params (ControlMessage :type Control%20Message%20Base%20Structure%20%28by%20ref%29))
  (Development|PrintString (Utilities|String|ToString(Integer) (Class|VICharacterBase|GetBlendPoseIDbyActionName (.bodylanguage (.speakpayload ControlMessage))))))

(event EventBeginPlay
  (bind _returnvalue (Rendering|Material|CreateDynamicMaterialInstance (Variables|Default|GetFaceScreen) 0 "/Game/VI_LS/Jimbo/JimboMaterials/M_FaceScreen.M_FaceScreen" "None" :!class /Script/Engine.PrimitiveComponent))
  (Variables|Default|SetFaceMat _returnvalue)
  (bind _asvi_game_instance (Utilities|Casting|CastToVI_GameInstance (Game|GetGameInstance)))
  (Variables|Default|SetVI_GameInstance _asvi_game_instance)
  (Utilities|FlowControl|Sequence
    (:then_0
      (EventDispatchers|BindEventtoOnControlMessage (Variables|Default|GetVI_GameInstance) (delegate Custom|OnCtrl)))
    (:then_1
      (EventDispatchers|BindEventtoOnTTSFeedback (Variables|Default|GetVI_GameInstance) (delegate Custom|TTSFeedback)))
    (:then_2
      (EventDispatchers|AssignOnWebsocketConnect (Variables|Default|GetVI_GameInstance) (delegate Custom|OnConnect)))))

(event Collision|EventActorBeginOverlap
  (params (OtherActor :type Actor%20Object%20Reference)))

(event EventTick
  (params (DeltaSeconds :type Float%20%28single-precision%29))
  (Rendering|Material|SetTextureParameterValue (Variables|Default|GetFaceMat) "ScreenWidget" (Class|WidgetComponent|GetRenderTarget (Variables|Default|GetFaceWidget))))

(fn ConstructionScript)