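; BP_VolumeBar is an actor that moves its Cube in a straight line and removes itself on reaching an end point.
; Tick shifts the Cube along Direction at Speed, scaled by delta time, and destroys the actor once the Cube is near FinishAt.
; The Jimbo VolumeOutput event is empty, and both the timed self-destroy and the construction-script BP_Jimbo lookup are disconnected.
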(event VolumeOutput(Jimbo)
  (params (EnvelopeValue :type Float%20%28double-precision%29)))

(event EventBeginPlay)

(event Collision|EventActorBeginOverlap
  (params (OtherActor :type Actor%20Object%20Reference)))

(event EventTick
  (params (DeltaSeconds :type Float%20%28single-precision%29))
  (bind _cube (Variables|Default|GetCube))
  (bind _returnvalue (Transformation|GetWorldLocation _cube))
  (Transformation|SetWorldLocation _cube (+ _returnvalue (* (* DeltaSeconds (Variables|Default|GetDirection)) (Variables|Default|GetSpeed))) false false)
  (if (< (Math|Vector|Distance(Vector) _returnvalue (Variables|Default|GetFinishAt)) 5e+01)
    (Actor|DestroyActor)))

(fn ConstructionScript)