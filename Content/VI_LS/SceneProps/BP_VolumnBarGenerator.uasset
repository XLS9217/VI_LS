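; BP_VolumnBarGenerator is a scene prop that spawns a stream of volume bars to visualize the audio level reported by BP_Jimbo.
; The construction script takes the first BP_Jimbo found, whose VolumeOutput event updates a stored envelope value.
; From BeginPlay, a repeating Delay loop spawns a BP_VolumeBar at Start, height-scaled by that envelope, and passes it a direction and finish point toward End.
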(event VolumeOutput(Jimbo)
  (params (EnvelopeValue :type Float%20%28double-precision%29))
  (Variables|Default|SetEnvelope%20Value EnvelopeValue))

(event EventBeginPlay
  (Variables|Default|SetStartLocation (Transformation|GetWorldLocation (Variables|Default|GetStart)))
  (Variables|Default|SetEndLocation (Transformation|GetWorldLocation (Variables|Default|GetEnd)))
  (Variables|Default|SetDirection (- "" (Math|Vector|Normalize (- (Variables|Default|GetStartLocation) (Variables|Default|GetEndLocation)))))
  (bind _returnvalue (Game|SpawnActorfromClass "/Game/VI_LS/SceneProps/BP_VolumeBar.BP_VolumeBar_C" (Math|Transform|MakeTransform (Variables|Default|GetStartLocation) "0, 0, 0" (Math|Vector|MakeVector 0.1 0.1 (+ (* (Variables|Default|GetEnvelope%20Value) 1e+01) 0.1))) "Undefined" "MultiplyWithRoot" 0 0 :!label _label))
  (Variables|/Game/VI_LS/SceneProps/BP_VolumeBar.BP_VolumeBar_C|SetDirection _returnvalue (Variables|Default|GetDirection))
  (Variables|/Game/VI_LS/SceneProps/BP_VolumeBar.BP_VolumeBar_C|SetFinishAt _returnvalue (Variables|Default|GetEndLocation))
  (Utilities|FlowControl|Delay 0.2)
  (goto _label))

(event Collision|EventActorBeginOverlap
  (params (OtherActor :type Actor%20Object%20Reference)))

(event EventTick
  (params (DeltaSeconds :type Float%20%28single-precision%29)))

(fn ConstructionScript
  (bind _outactors (Actor|GetAllActorsOfClass "/Game/VI_LS/Jimbo/BP_Jimbo.BP_Jimbo_C"))
  (for (_array_element _array_index) _outactors
    (if (== _array_index 0)
      (Variables|Default|SetJimbo _array_element))))